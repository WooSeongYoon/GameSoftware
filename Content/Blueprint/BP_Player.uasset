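; BP_Player is a player actor that moves in the Y-Z plane and fires bullets.
; BeginPlay adds the IMC_PlayerInput Enhanced Input mapping context, and horizontal and vertical actions store their axis values.
; Tick adds those values directly to the actor location each frame, without sweep or delta-time scaling.
; The fire action spawns a BP_Bullet at the FirePosition component's transform.
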(event Input|EnhancedActionEvents|EnhancedInputActionIA_Fire
  (params (ActionValue :type Boolean) (ElapsedSeconds :type Float%20%28double-precision%29) (TriggeredSeconds :type Float%20%28double-precision%29) (InputAction :type Input%20Action%20Object%20Reference :default "/Game/Inouts/IA_Fire.IA_Fire"))
  (:Started
    (Game|SpawnActorfromClass "/Game/Blueprint/BP_Bullet.BP_Bullet_C" (Transformation|GetWorldTransform (Variables|Default|GetFirePosition)) "AlwaysSpawn" "MultiplyWithRoot" 0 0)))

(event Input|EnhancedActionEvents|EnhancedInputActionIA_Horizotal
  (params (ActionValue :type Float%20%28double-precision%29) (ElapsedSeconds :type Float%20%28double-precision%29) (TriggeredSeconds :type Float%20%28double-precision%29) (InputAction :type Input%20Action%20Object%20Reference :default "/Game/Inouts/IA_Horizotal.IA_Horizotal"))
  (:Triggered
    (Variables|Default|SetHorizeontal ActionValue))
  (:Completed
    (Variables|Default|SetHorizeontal ActionValue)))

(event Input|EnhancedActionEvents|EnhancedInputActionIA_Vertical
  (params (ActionValue :type Float%20%28double-precision%29) (ElapsedSeconds :type Float%20%28double-precision%29) (TriggeredSeconds :type Float%20%28double-precision%29) (InputAction :type Input%20Action%20Object%20Reference :default "/Game/Inouts/IA_Vertical.IA_Vertical"))
  (:Triggered
    (Variables|Default|SetVertical ActionValue))
  (:Completed
    (Variables|Default|SetVertical ActionValue)))

(event EventBeginPlay
  (Input|AddMappingContext (PlayerController|LocalPlayerSubsystems|GetEnhancedInputLocalPlayerSubsystem (Game|GetPlayerController 0)) "/Game/Inouts/IMC_PlayerInput.IMC_PlayerInput" 0 "(bIgnoreAllPressedKeysUntilRelease=True,bForceImmediately=False,bNotifyUserSettings=False)"))

(event EventTick
  (params (DeltaSeconds :type Float%20%28single-precision%29))
  (Transformation|SetActorLocation (+ (Transformation|GetActorLocation) (Math|Vector|MakeVector 0.0 (Variables|Default|GetHorizeontal) (Variables|Default|GetVertical))) false false))

(fn ConstructionScript)