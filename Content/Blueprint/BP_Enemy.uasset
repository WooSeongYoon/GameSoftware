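; BP_Enemy is an enemy actor that flies in a straight line and ends the game when it touches BP_Player.
; On BeginPlay a random roll against TraceRate either aims it once at the player's current position or keeps its forward vector.
; Tick moves it along that fixed direction at MoveSpeed without sweeping.
; Overlap destroys the player, spawns blood, shows the game-over widget and cursor, and pauses.
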(event EventBeginPlay
  (if (<= (Math|Random|RandomFloatinRange 0.0 1.0) (Variables|Default|GetTraceRate))
    (bind _returnvalue (Actor|GetActorOfClass "/Game/Blueprint/BP_Player.BP_Player_C"))
    (Utilities|IsValid _returnvalue
      (:Is%20Valid
        (bind _output_get (Variables|Default|SetDirection (Math|Vector|Normalize (- (Transformation|GetActorLocation _returnvalue) (Transformation|GetActorLocation)))))
        (Transformation|SetActorRotation (Math|Rotator|MakeRotfromXZ _output_get (Transformation|GetActorUpVector)))))
    (else
      (Variables|Default|SetDirection (Transformation|GetActorForwardVector)))))

(event Collision|EventActorBeginOverlap
  (params (OtherActor :type Actor%20Object%20Reference))
  (bind _asbp_player (Utilities|Casting|CastToBP_Player OtherActor))
  (Actor|DestroyActor _asbp_player)
  (Effects|SpawnEmitteratLocation "/Game/Realistic_Starter_VFX_Pack_Vol2/Particles/Blood/P_Blood_Splat_Cone.P_Blood_Splat_Cone" (Transformation|GetActorLocation))
  (bind _returnvalue (UserInterface|CreateWidget "/Game/UI/WBP_GameOverWidgt.WBP_GameOverWidgt_C"))
  (UserInterface|Viewport|AddtoViewport _returnvalue 0)
  (Variables|/Script/Engine.PlayerController|SetbShowMouseCursor (Game|GetPlayerController 0) true)
  (Game|SetGamePaused true))

(event EventTick
  (params (DeltaSeconds :type Float%20%28single-precision%29))
  ;[1 1 1] Enemy Move
  (Transformation|SetActorLocation (+ (* DeltaSeconds (* (Variables|Default|GetDirection) (Variables|Default|GetMoveSpeed))) (Transformation|GetActorLocation)) false false))

(fn ConstructionScript)